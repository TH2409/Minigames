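; BP_Curtains is a multi-piece curtain actor that animates itself closed when its Close event is called.
; Close starts four timelines together through a Sequence, each lerping relative transforms of static mesh pieces.
; The top piece swings, the main halves slide inward, side pieces drop, and tied curtains rotate and rise.
; It only plays forward, with no opening logic in the graph.
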(event `Close`
  (`|ExecutionSequence`
    (:`then_0`
      ;[1 1 1] Top
      (bind (_direction _newtrack_0) (`Timeline|TopSwing`)
        (:`Update`
          (`SceneComponent.K2_SetRelativeRotation` (`self.SM_CurtainTop`) (`KismetMathLibrary.MakeRotator` (`KismetMathLibrary.Lerp` 360.0 180.0 _newtrack_0)) false false))))
    (:`then_1`
      ;[1 1 1] Main
      (bind (_direction_2 _newtrack_1) (`Timeline|MainCurtains`)
        (:`Update`
          (`SceneComponent.K2_SetRelativeLocation` (`self.SM_CurtainLeft`) (`KismetMathLibrary.VLerp` (-100.0 -6.31581 0.0) (5.0 -6.31581 0.0) _newtrack_1) false false)
          (`SceneComponent.K2_SetRelativeLocation` (`self.SM_CurtainRight`) (`KismetMathLibrary.VLerp` (100.0 -4.704722 0.0) (-5.0 -4.704722 0.0) _newtrack_1) false false))))
    (:`then_2`
      ;[1 1 1] Extras
      (bind (_direction_3 _newtrack_2) (`Timeline|SidesDrop`)
        (:`Update`
          (`SceneComponent.K2_SetRelativeLocation` (`self.SM_CurtainLeftSide`) (`KismetMathLibrary.VLerp` (-71.801697 3.212799 100.0) (-66.801697 3.212799 0.0) _newtrack_2) false false)
          (`SceneComponent.K2_SetRelativeLocation` (`self.SM_CurtainRightSide`) (`KismetMathLibrary.VLerp` (70.928391 3.212799 100.0) (65.928391 3.212799 0.0) _newtrack_2) false false))))
    (:`then_3`
      ;[1 1 1] TiedCurtains
      (bind (_direction_4 _newtrack_0_2) (`Timeline|TiedCurtainsRotate`)
        (:`Update`
          (`SceneComponent.K2_SetRelativeRotation` (`self.SM_CurtainRightTied`) (`KismetMathLibrary.MakeRotator` 0.0 (`KismetMathLibrary.Lerp` 0.0 90.0 _newtrack_0_2)) false false)
          (`SceneComponent.K2_SetRelativeRotation` (`self.SM_CurtainLeftTied`) (`KismetMathLibrary.MakeRotator` 0.0 (`KismetMathLibrary.Lerp` 0.0 -90.0 _newtrack_0_2)) false false)
          (`SceneComponent.K2_SetRelativeLocation` (`self.SM_CurtainRightTied`) (`KismetMathLibrary.VLerp` (35.703545 0.00018 0.0) (35.703545 0.00018 40.0) _newtrack_0_2) false false)
          (`SceneComponent.K2_SetRelativeLocation` (`self.SM_CurtainLeftTied`) (`KismetMathLibrary.VLerp` (-38.933071 -0.001083 0.0) (-38.933071 -0.001083 40.0) _newtrack_0_2) false false))))))

(fn `UserConstructionScript`)