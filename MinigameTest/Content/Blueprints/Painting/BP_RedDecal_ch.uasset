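; BP_RedDecal_ch is a red paint decal actor that can be wiped away by a cleaning painting object.
; The construction script creates a dynamic decal material and assigns a random stroke alpha texture from an array for variety.
; A box overlap checks for a C_Painting actor and destroys the decal when that actor's Clean flag is set.
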(event `self.Box.OnComponentBeginOverlap`
  (params (OverlappedComponent :type "PrimitiveComponent Object Reference") (OtherActor :type "Actor Object Reference") (OtherComp :type "PrimitiveComponent Object Reference") (OtherBodyIndex :type Integer) (bFromSweep :type Boolean) (SweepResult :type "HitResult Structure (by ref)"))
  (bind _asc_painting (cast `/Game/Characters/C_Painting` OtherActor))
  (if (`/Game/Characters/C_Painting.clean` _asc_painting)
    (`self.K2_DestroyActor`)))

(fn `UserConstructionScript`
  (bind _paintalphas (`self.PaintAlphas`))
  (bind _returnvalue (`DecalComponent.CreateDynamicMaterialInstance` (`self.Decal`)))
  (bind _output_get (set `self.DecalMaterial` _returnvalue))
  (`MaterialInstanceDynamic.SetTextureParameterValue` _output_get "StrokeType" (`|GetArrayItem` _paintalphas (`KismetMathLibrary.RandomInteger` (`KismetArrayLibrary.Array_Length` _paintalphas)))))