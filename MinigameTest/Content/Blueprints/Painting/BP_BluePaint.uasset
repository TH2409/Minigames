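; Blue paint actor that turns into a floor splat after something overlaps its Sphere1 component.
; One second after overlap, it spawns BP_BlueDecal at the Sphere's XY with Z zero, randomizing rotation and scale for variety.
; Scale selects use RandomInteger(1), which always returns zero, so only the negative ranges apply.
; A DoOnce then plays one of four random splat sounds and destroys the actor.
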(event `self.Sphere1.OnComponentBeginOverlap`
  (params (OverlappedComponent :type "PrimitiveComponent Object Reference") (OtherActor :type "Actor Object Reference") (OtherComp :type "PrimitiveComponent Object Reference") (OtherBodyIndex :type Integer) (bFromSweep :type Boolean) (SweepResult :type "HitResult Structure (by ref)"))
  (bind (_returnvalue_x _returnvalue_y) (`KismetMathLibrary.BreakVector` (`SceneComponent.K2_GetComponentLocation` (`self.Sphere`))))
  (bind _returnvalue (select `int` (`KismetMathLibrary.RandomInteger` 1) :`0` (`KismetMathLibrary.RandomFloatInRange` -1.0 -0.8) :`1` (`KismetMathLibrary.RandomFloatInRange` 0.8 1.0)))
  (`KismetSystemLibrary.Delay` 1.0)
  (`|SpawnActorFromClass` "/Game/Blueprints/Painting/BP_BlueDecal.BP_BlueDecal_C" (`KismetMathLibrary.MakeTransform` (`KismetMathLibrary.MakeVector` _returnvalue_x _returnvalue_y) (`KismetMathLibrary.MakeRotator` (`KismetMathLibrary.RandomFloatInRange` 0.0 30.0) 0.0 (`KismetMathLibrary.RandomFloatInRange` 0.0 360.0)) (`KismetMathLibrary.MakeVector` _returnvalue _returnvalue _returnvalue)) "Undefined" "OverrideRootScale")
  (`/Engine/EditorBlueprintResources/StandardMacros.DoOnce` false
    (:`Completed`
      (switch `int` (`KismetMathLibrary.RandomInteger` 4)
        (:`0`
          (`GameplayStatics.PlaySound2D` "/Game/Audio/Painting/PaintSplat1.PaintSplat1"))
        (:`1`
          (`GameplayStatics.PlaySound2D` "/Game/Audio/Painting/PaintSplat2.PaintSplat2"))
        (:`2`
          (`GameplayStatics.PlaySound2D` "/Game/Audio/Painting/PaintSplat3.PaintSplat3"))
        (:`3`
          (`GameplayStatics.PlaySound2D` "/Game/Audio/Painting/PaintSplat4.PaintSplat4")))
      (`self.K2_DestroyActor`))))

(fn `UserConstructionScript`)