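; BP_SandwichSpawner periodically spawns sandwich ingredients at its own location.
; A looping half-second timer set on BeginPlay calls Spawn, which acts only while the Start flag is true.
; A six-way random roll picks Bread, Meat or Veg at reduced scale, and the three unhandled outcomes spawn nothing, so about half the ticks stay empty.
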(event `self.ReceiveBeginPlay`
  (`KismetSystemLibrary.K2_SetTimer` null "Spawn" 0.5 true))

(event `Spawn`
  (if (`self.start?`)
    (switch `int` (`KismetMathLibrary.RandomInteger` 6)
      (:`0`
        (`|SpawnActorFromClass` "/Game/Blueprints/Sandwich/Bread.Bread_C" (`KismetMathLibrary.MakeTransform` (`self.K2_GetActorLocation`) (struct) (0.4 0.4 0.4)) "Undefined" "OverrideRootScale"))
      (:`1`
        (`|SpawnActorFromClass` "/Game/Blueprints/Sandwich/Meat.Meat_C" (`KismetMathLibrary.MakeTransform` (`self.K2_GetActorLocation`) (struct) (0.4 0.4 0.4)) "Undefined" "OverrideRootScale"))
      (:`2`
        (`|SpawnActorFromClass` "/Game/Blueprints/Sandwich/Veg.Veg_C" (`KismetMathLibrary.MakeTransform` (`self.K2_GetActorLocation`) (struct) (0.4 0.4 0.4)) "Undefined" "OverrideRootScale")))))

(fn `UserConstructionScript`)