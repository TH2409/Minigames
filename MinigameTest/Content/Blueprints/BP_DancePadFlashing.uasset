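; BP_DancePadFlashing is a dance pad actor whose material lights flash in an endless animated loop.
; The construction script creates a dynamic instance of the dance pad ball material and applies it to the pad mesh.
; On BeginPlay, a timeline drives its emissive opacity, Cross and Plus scalar parameters, then restarts from the start whenever it finishes.
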(event `self.ReceiveBeginPlay`
  (bind _padmaterial (`self.PadMaterial`))
  (bind (_direction _lightopacity _lights1 _lights2 _lights3) (`Timeline|Timeline_0` :!label _label)
    (:`Update`
      (`|ExecutionSequence`
        (:`then_0`
          (`MaterialInstanceDynamic.SetScalarParameterValue` _padmaterial "EmissOpacity" _lightopacity))
        (:`then_2`
          (`MaterialInstanceDynamic.SetScalarParameterValue` _padmaterial "Cross" _lights2))
        (:`then_3`
          (`MaterialInstanceDynamic.SetScalarParameterValue` _padmaterial "Plus" _lights3))))
    (:`Finished`
      (`self.Repeat`
        (:`Out`
          (goto _label :!via `PlayFromStart`))))))

(fn `UserConstructionScript`
  (bind _returnvalue (`PrimitiveComponent.CreateDynamicMaterialInstance` (`self.SM_DancePad`) 0 "/Game/Materials/M_DancePadBall_MI.M_DancePadBall_MI"))
  (set `self.PadMaterial` _returnvalue)
  (`PrimitiveComponent.SetMaterial` (`self.SM_DancePad`) 0 (`self.PadMaterial`)))