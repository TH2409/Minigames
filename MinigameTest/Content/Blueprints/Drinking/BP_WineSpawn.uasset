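; BP_WineSpawn is a wine pour emitter that spawns BP_Wine actors at its root location.
; While On is true, every Tick re-sets a looping 0.02-second timer for the spawn event, and nothing here clears it.
; Each spawn call creates one wine actor, and the first also plays a pour-start sound followed by a delayed pour-loop sound through a DoOnce that is never reset.
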(event `self.ReceiveTick`
  (params (DeltaSeconds :type "Float (single-precision)"))
  (if (`self.on?`)
    (`KismetSystemLibrary.K2_SetTimer` null "spawn" 0.02 true)))

(event `spawn`
  (`|ExecutionSequence`
    (:`then_0`
      (`/Engine/EditorBlueprintResources/StandardMacros.DoOnce` false
        (:`Completed`
          (`GameplayStatics.PlaySound2D` "/Game/Audio/Drinking/WinePourStart.WinePourStart")
          (`KismetSystemLibrary.Delay` 1.46)
          (`GameplayStatics.PlaySound2D` "/Game/Audio/Drinking/WinePourLoop.WinePourLoop"))))
    (:`then_1`
      (`|SpawnActorFromClass` "/Game/Blueprints/Drinking/BP_Wine.BP_Wine_C" (`KismetMathLibrary.Conv_VectorToTransform` (`SceneComponent.K2_GetComponentLocation` (`self.DefaultSceneRoot`))) "Undefined" "OverrideRootScale"))))

(fn `UserConstructionScript`)