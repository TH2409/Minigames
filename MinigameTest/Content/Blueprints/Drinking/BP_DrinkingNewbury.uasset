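; BP_DrinkingNewbury is a Blueprint that scores drinking objects overlapping its box trigger.
; An overlap counts when the other component is a C_Drinking actor's own Box and that actor's display name matches the stored Name.
; It then plays a timeline that pitches StaticMesh1 and adds the drink's Number to Points.
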(event `self.Box.OnComponentBeginOverlap`
  (params (OverlappedComponent :type "PrimitiveComponent Object Reference") (OtherActor :type "Actor Object Reference") (OtherComp :type "PrimitiveComponent Object Reference") (OtherBodyIndex :type Integer) (bFromSweep :type Boolean) (SweepResult :type "HitResult Structure (by ref)"))
  (if (and (== (`/Game/Characters/C_Drinking.Box` (cast `/Game/Characters/C_Drinking` OtherActor :!pure true)) OtherComp) (`KismetStringLibrary.EqualEqual_StrStr` (`KismetSystemLibrary.GetDisplayName` OtherActor) (`self.Name`)))
    (`|ExecutionSequence`
      (:`then_0`
        (bind (_direction _newtrack_0) (`Timeline|Timeline_0` :!via `PlayFromStart`)
          (:`Update`
            (`SceneComponent.K2_SetRelativeRotation` (`self.StaticMesh1`) (`KismetMathLibrary.MakeRotator` 0.0 _newtrack_0) false false))))
      (:`then_1`
        (bind _asc_drinking (cast `/Game/Characters/C_Drinking` OtherActor))
        (set `self.points` (+ (`self.points`) (`/Game/Characters/C_Drinking.number` _asc_drinking)))))))

(fn `UserConstructionScript`)