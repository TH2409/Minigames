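; Cutting station for the cooking game that advances each chef's ingredient to its prepared state on overlapping its box.
; Begin overlap casts to six character classes, swaps their ingredient booleans and starts a matching cutting, spooning, buttering or scraping audio cue.
; Reginald's branch differs, re-setting CookedChicken and clearing Chicken instead of setting a new prepared flag.
; Any end overlap stops all four cues, whichever actor leaves.
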(event `self.Box.OnComponentBeginOverlap`
  (params (OverlappedComponent :type "PrimitiveComponent Object Reference") (OtherActor :type "Actor Object Reference") (OtherComp :type "PrimitiveComponent Object Reference") (OtherBodyIndex :type Integer) (bFromSweep :type Boolean) (SweepResult :type "HitResult Structure (by ref)"))
  (`|ExecutionSequence`
    (:`then_0`
      (bind _asc_cooking_newbury (cast `/Game/Characters/C_CookingNewbury` OtherActor))
      (if (`/Game/Characters/C_CookingNewbury.Eels` _asc_cooking_newbury)
        (`|ExecutionSequence`
          (:`then_0`
            (set `/Game/Characters/C_CookingNewbury.CutEels` true _asc_cooking_newbury)
            (set `/Game/Characters/C_CookingNewbury.Eels` false _asc_cooking_newbury))
          (:`then_1`
            (`AudioComponent.Play` (`self.CuttingLoop_Cue`) 0.0 :!label _label)))))
    (:`then_1`
      (bind _asc_cooking_reginald (cast `/Game/Characters/C_CookingReginald` OtherActor))
      (if (`/Game/Characters/C_CookingReginald.Cooked Chicken` _asc_cooking_reginald)
        (`|ExecutionSequence`
          (:`then_0`
            (set `/Game/Characters/C_CookingReginald.Cooked Chicken` true _asc_cooking_reginald)
            (set `/Game/Characters/C_CookingReginald.Chicken` false _asc_cooking_reginald))
          (:`then_1`
            (goto _label)))))
    (:`then_2`
      (bind _asc_cooking_yvonne (cast `/Game/Characters/C_CookingYvonne` OtherActor))
      (if (`/Game/Characters/C_CookingYvonne.CookedCaviar` _asc_cooking_yvonne)
        (`|ExecutionSequence`
          (:`then_0`
            (set `/Game/Characters/C_CookingYvonne.SpoonedCaviar` true _asc_cooking_yvonne)
            (set `/Game/Characters/C_CookingYvonne.CookedCaviar` false _asc_cooking_yvonne))
          (:`then_1`
            (`AudioComponent.Play` (`self.SpooningLoop_Cue`) 0.0)))))
    (:`then_3`
      (bind _asc_cooking_chad (cast `/Game/Characters/C_CookingChad` OtherActor))
      (if (`/Game/Characters/C_CookingChad.CookedLobster` _asc_cooking_chad)
        (`|ExecutionSequence`
          (:`then_0`
            (set `/Game/Characters/C_CookingChad.ButteredLobster` true _asc_cooking_chad)
            (set `/Game/Characters/C_CookingChad.CookedLobster` false _asc_cooking_chad))
          (:`then_1`
            (`AudioComponent.Play` (`self.ButteringLoop_Cue`) 0.0)))))
    (:`then_4`
      (bind _asc_cooking_jeremia (cast `/Game/Characters/C_CookingJeremia` OtherActor))
      (if (`/Game/Characters/C_CookingJeremia.Smelt Cheese` _asc_cooking_jeremia)
        (`|ExecutionSequence`
          (:`then_0`
            (set `/Game/Characters/C_CookingJeremia.Cut Cheese` true _asc_cooking_jeremia)
            (set `/Game/Characters/C_CookingJeremia.Smelt Cheese` false _asc_cooking_jeremia))
          (:`then_1`
            (goto _label)))))
    (:`then_5`
      (bind _asc_cooking_diana (cast `/Game/Characters/C_CookingDiana` OtherActor))
      (if (`/Game/Characters/C_CookingDiana.Cooked Snails` _asc_cooking_diana)
        (`|ExecutionSequence`
          (:`then_0`
            (set `/Game/Characters/C_CookingDiana.Scraped Snails` true _asc_cooking_diana)
            (set `/Game/Characters/C_CookingDiana.Cooked Snails` false _asc_cooking_diana))
          (:`then_1`
            (`AudioComponent.Play` (`self.ScrapingLoop_Cue`) 0.0)))))))

(event `self.Box.OnComponentEndOverlap`
  (params (OverlappedComponent :type "PrimitiveComponent Object Reference") (OtherActor :type "Actor Object Reference") (OtherComp :type "PrimitiveComponent Object Reference") (OtherBodyIndex :type Integer))
  (`AudioComponent.Stop` (`self.CuttingLoop_Cue`))
  (`AudioComponent.Stop` (`self.ButteringLoop_Cue`))
  (`AudioComponent.Stop` (`self.SpooningLoop_Cue`))
  (`AudioComponent.Stop` (`self.ScrapingLoop_Cue`)))

(fn `UserConstructionScript`)