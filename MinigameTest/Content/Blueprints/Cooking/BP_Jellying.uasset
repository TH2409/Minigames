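; BP_Jellying is a cooking station that turns a player's cut eels into jellied eels when they step into its trigger box.
; On box overlap, it casts the actor to C_CookingNewbury and, if CutEels is set, swaps that flag for JelliesEels and plays a looping jellying sound.
; Any end overlap on the box stops the sound.
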(event `self.Box.OnComponentBeginOverlap`
  (params (OverlappedComponent :type "PrimitiveComponent Object Reference") (OtherActor :type "Actor Object Reference") (OtherComp :type "PrimitiveComponent Object Reference") (OtherBodyIndex :type Integer) (bFromSweep :type Boolean) (SweepResult :type "HitResult Structure (by ref)"))
  (bind _asc_cooking_newbury (cast `/Game/Characters/C_CookingNewbury` OtherActor))
  (if (`/Game/Characters/C_CookingNewbury.CutEels` _asc_cooking_newbury)
    (`|ExecutionSequence`
      (:`then_0`
        (set `/Game/Characters/C_CookingNewbury.JelliesEels` true _asc_cooking_newbury)
        (set `/Game/Characters/C_CookingNewbury.CutEels` false _asc_cooking_newbury))
      (:`then_1`
        (`AudioComponent.Play` (`self.JellyingLoop_Cue`) 0.0)))))

(event `self.Box.OnComponentEndOverlap`
  (params (OverlappedComponent :type "PrimitiveComponent Object Reference") (OtherActor :type "Actor Object Reference") (OtherComp :type "PrimitiveComponent Object Reference") (OtherBodyIndex :type Integer))
  (`AudioComponent.Stop` (`self.JellyingLoop_Cue`)))

(fn `UserConstructionScript`)