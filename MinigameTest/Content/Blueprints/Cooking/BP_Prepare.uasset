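; BP_Prepare is a cooking station that turns processed ingredients into prepared ones when a C_Cooking actor overlaps its box.
; Cooked potatoes, cut beef and cooked veg each have their flag on that actor swapped for the matching prepared flag.
; A final check in the same sequence sets FullMeal once all three are prepared, with debug strings printed at each change.
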(event `self.Box.OnComponentBeginOverlap`
  (params (OverlappedComponent :type "PrimitiveComponent Object Reference") (OtherActor :type "Actor Object Reference") (OtherComp :type "PrimitiveComponent Object Reference") (OtherBodyIndex :type Integer) (bFromSweep :type Boolean) (SweepResult :type "HitResult Structure (by ref)"))
  (bind _asc_cooking (cast `/Game/Characters/C_Cooking` OtherActor))
  (`|ExecutionSequence`
    (:`then_0`
      (if (`/Game/Characters/C_Cooking.Cooked potatoes` _asc_cooking)
        (set `/Game/Characters/C_Cooking.Prepared potatoes` true _asc_cooking)
        (set `/Game/Characters/C_Cooking.Cooked potatoes` false _asc_cooking)
        (`KismetSystemLibrary.PrintString` "Prepared Potatoes")))
    (:`then_1`
      (if (`/Game/Characters/C_Cooking.Cut beef` _asc_cooking)
        (set `/Game/Characters/C_Cooking.Prepared beef` true _asc_cooking)
        (set `/Game/Characters/C_Cooking.Cut beef` false _asc_cooking)
        (`KismetSystemLibrary.PrintString` "Prepared Beef")))
    (:`then_2`
      (if (`/Game/Characters/C_Cooking.Cooked veg` _asc_cooking)
        (set `/Game/Characters/C_Cooking.Prepared veg` true _asc_cooking)
        (set `/Game/Characters/C_Cooking.Cooked veg` false _asc_cooking)
        (`KismetSystemLibrary.PrintString` "Prepared Veg")))
    (:`then_3`
      (if (and (`/Game/Characters/C_Cooking.Prepared beef` _asc_cooking) (`/Game/Characters/C_Cooking.Prepared potatoes` _asc_cooking) (`/Game/Characters/C_Cooking.Prepared veg` _asc_cooking))
        (set `/Game/Characters/C_Cooking.Full meal` true _asc_cooking)
        (`KismetSystemLibrary.PrintString` "Full Meal")))))

(fn `UserConstructionScript`)