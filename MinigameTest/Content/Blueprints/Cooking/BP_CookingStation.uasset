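; BP_CookingStation is a hob/oven that cooks each character's ingredient when they step into its trigger Box.
; On overlap it casts to Reginald, Yvonne, Chad or Diana and swaps their raw chicken, uncanned caviar, lobster or snails flag for the cooked one.
; A successful cook starts a boiling sound loop and a timeline that rolls the oven mesh.
; Any end overlap stops the sound.
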(event `self.Box.OnComponentBeginOverlap`
  (params (OverlappedComponent :type "PrimitiveComponent Object Reference") (OtherActor :type "Actor Object Reference") (OtherComp :type "PrimitiveComponent Object Reference") (OtherBodyIndex :type Integer) (bFromSweep :type Boolean) (SweepResult :type "HitResult Structure (by ref)"))
  (`|ExecutionSequence`
    (:`then_0`
      (bind _asc_cooking_reginald (cast `/Game/Characters/C_CookingReginald` OtherActor))
      (if (`/Game/Characters/C_CookingReginald.Chicken` _asc_cooking_reginald)
        (`|ExecutionSequence`
          (:`then_0`
            (set `/Game/Characters/C_CookingReginald.Cooked Chicken` true _asc_cooking_reginald)
            (set `/Game/Characters/C_CookingReginald.Chicken` false _asc_cooking_reginald))
          (:`then_1`
            (`AudioComponent.Play` (`self.BoilingLoop_Cue`) 0.0))
          (:`then_2`
            (bind (_direction _newtrack_0) (`Timeline|Timeline_0` :!via `PlayFromStart` :!label _label)
              (:`Update`
                (`SceneComponent.K2_SetRelativeRotation` (`self.SM_HobOven1`) (`KismetMathLibrary.MakeRotator` _newtrack_0) false false)))))))
    (:`then_1`
      (bind _asc_cooking_yvonne (cast `/Game/Characters/C_CookingYvonne` OtherActor))
      (if (`/Game/Characters/C_CookingYvonne.UncannedCaviar` _asc_cooking_yvonne)
        (`|ExecutionSequence`
          (:`then_0`
            (set `/Game/Characters/C_CookingYvonne.CookedCaviar` true _asc_cooking_yvonne)
            (set `/Game/Characters/C_CookingYvonne.UncannedCaviar` false _asc_cooking_yvonne))
          (:`then_1`
            (`AudioComponent.Play` (`self.BoilingLoop_Cue`) 0.0))
          (:`then_2`
            (goto _label :!via `PlayFromStart`)))))
    (:`then_2`
      (bind _asc_cooking_chad (cast `/Game/Characters/C_CookingChad` OtherActor))
      (if (`/Game/Characters/C_CookingChad.Lobster` _asc_cooking_chad)
        (`|ExecutionSequence`
          (:`then_0`
            (set `/Game/Characters/C_CookingChad.CookedLobster` true _asc_cooking_chad)
            (set `/Game/Characters/C_CookingChad.Lobster` false _asc_cooking_chad))
          (:`then_1`
            (`AudioComponent.Play` (`self.BoilingLoop_Cue`) 0.0))
          (:`then_2`
            (goto _label :!via `PlayFromStart`)))))
    (:`then_3`
      (bind _asc_cooking_diana (cast `/Game/Characters/C_CookingDiana` OtherActor))
      (if (`/Game/Characters/C_CookingDiana.Snails` _asc_cooking_diana)
        (`|ExecutionSequence`
          (:`then_0`
            (set `/Game/Characters/C_CookingDiana.Cooked Snails` true _asc_cooking_diana)
            (set `/Game/Characters/C_CookingDiana.Snails` false _asc_cooking_diana))
          (:`then_1`
            (`AudioComponent.Play` (`self.BoilingLoop_Cue`) 0.0))
          (:`then_2`
            (goto _label :!via `PlayFromStart`)))))))

(event `self.Box.OnComponentEndOverlap`
  (params (OverlappedComponent :type "PrimitiveComponent Object Reference") (OtherActor :type "Actor Object Reference") (OtherComp :type "PrimitiveComponent Object Reference") (OtherBodyIndex :type Integer))
  (`AudioComponent.Stop` (`self.BoilingLoop_Cue`)))

(fn `UserConstructionScript`)