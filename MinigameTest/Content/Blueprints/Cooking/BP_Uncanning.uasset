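; BP_Uncanning is a cooking station that gives Yvonne uncanned caviar when she walks into it empty-handed.
; Box overlap with C_CookingYvonne, if her Empty flag is set, marks her as holding UncannedCaviar, plays DeCanningCue and shows the can mesh for three seconds.
; Leaving the box stops the sound, while Tick spins the can mesh continuously.
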(event `self.ReceiveTick`
  (params (DeltaSeconds :type "Float (single-precision)"))
  (`SceneComponent.K2_AddLocalRotation` (`self.SM_Can`) (struct :`Yaw` -1.0) false false))

(event `self.Box.OnComponentBeginOverlap`
  (params (OverlappedComponent :type "PrimitiveComponent Object Reference") (OtherActor :type "Actor Object Reference") (OtherComp :type "PrimitiveComponent Object Reference") (OtherBodyIndex :type Integer) (bFromSweep :type Boolean) (SweepResult :type "HitResult Structure (by ref)"))
  (bind _sm_can (`self.SM_Can`))
  (bind _asc_cooking_yvonne (cast `/Game/Characters/C_CookingYvonne` OtherActor))
  (if (`/Game/Characters/C_CookingYvonne.Empty` _asc_cooking_yvonne)
    (`|ExecutionSequence`
      (:`then_0`
        (set `/Game/Characters/C_CookingYvonne.UncannedCaviar` true _asc_cooking_yvonne)
        (set `/Game/Characters/C_CookingYvonne.Empty` false _asc_cooking_yvonne))
      (:`then_1`
        (`AudioComponent.Play` (`self.DeCanning_Cue`) 0.0))
      (:`then_2`
        (`SceneComponent.SetVisibility` _sm_can true false)
        (`KismetSystemLibrary.Delay` 3.0)
        (`SceneComponent.SetVisibility` _sm_can false false)))))

(event `self.Box.OnComponentEndOverlap`
  (params (OverlappedComponent :type "PrimitiveComponent Object Reference") (OtherActor :type "Actor Object Reference") (OtherComp :type "PrimitiveComponent Object Reference") (OtherBodyIndex :type Integer))
  (`AudioComponent.Stop` (`self.DeCanning_Cue`)))

(fn `UserConstructionScript`)