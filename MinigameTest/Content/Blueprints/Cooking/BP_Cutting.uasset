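; BP_Cutting is a cooking station actor that chops the ingredients carried by a C_CookingNewbury.
; When an actor overlaps its Box, it casts to C_CookingNewbury and checks the flags for vegetables, potatoes and cooked beef.
; Each flag that is set is swapped for its cut counterpart, with a debug message printed on screen.
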(event `self.Box.OnComponentBeginOverlap`
  (params (OverlappedComponent :type "PrimitiveComponent Object Reference") (OtherActor :type "Actor Object Reference") (OtherComp :type "PrimitiveComponent Object Reference") (OtherBodyIndex :type Integer) (bFromSweep :type Boolean) (SweepResult :type "HitResult Structure (by ref)"))
  (bind _asc_cooking_newbury (cast `/Game/Characters/C_CookingNewbury` OtherActor))
  (`|ExecutionSequence`
    (:`then_0`
      (if (`/Game/Characters/C_CookingNewbury.Veg` _asc_cooking_newbury)
        (set `/Game/Characters/C_CookingNewbury.Cut veg` true _asc_cooking_newbury)
        (set `/Game/Characters/C_CookingNewbury.Veg` false _asc_cooking_newbury)
        (`KismetSystemLibrary.PrintString` "Cut Veg")))
    (:`then_1`
      (if (`/Game/Characters/C_CookingNewbury.Potatoes` _asc_cooking_newbury)
        (set `/Game/Characters/C_CookingNewbury.Cut potatoes` true _asc_cooking_newbury)
        (set `/Game/Characters/C_CookingNewbury.Potatoes` false _asc_cooking_newbury)
        (`KismetSystemLibrary.PrintString` "Cut Potatoes")))
    (:`then_2`
      (if (`/Game/Characters/C_CookingNewbury.Cooked beef` _asc_cooking_newbury)
        (set `/Game/Characters/C_CookingNewbury.Cut beef` true _asc_cooking_newbury)
        (set `/Game/Characters/C_CookingNewbury.Cooked beef` false _asc_cooking_newbury)
        (`KismetSystemLibrary.PrintString` "Cut Beef")))))

(fn `UserConstructionScript`)