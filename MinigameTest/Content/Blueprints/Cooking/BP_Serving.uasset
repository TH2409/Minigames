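; Serving station for the cooking game where characters turn in their finished dishes for points.
; On box overlap, a sequence tries casts to six character classes, each checked for its own dish flag, such as CutChicken or ButteredLobster.
; A match clears that flag, marks the character Empty, adds 100 to its Points and plays a plating sound.
; The logic is duplicated per character class rather than shared.
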(event `self.Box.OnComponentBeginOverlap`
  (params (OverlappedComponent :type "PrimitiveComponent Object Reference") (OtherActor :type "Actor Object Reference") (OtherComp :type "PrimitiveComponent Object Reference") (OtherBodyIndex :type Integer) (bFromSweep :type Boolean) (SweepResult :type "HitResult Structure (by ref)"))
  (`|ExecutionSequence`
    (:`then_0`
      (bind _asc_cooking_newbury (cast `/Game/Characters/C_CookingNewbury` OtherActor))
      (if (`/Game/Characters/C_CookingNewbury.JelliesEels` _asc_cooking_newbury)
        (set `/Game/Characters/C_CookingNewbury.JelliesEels` false _asc_cooking_newbury)
        (set `/Game/Characters/C_CookingNewbury.Empty` true _asc_cooking_newbury)
        (set `/Game/Characters/C_CookingNewbury.points` (+ (`/Game/Characters/C_CookingNewbury.points` _asc_cooking_newbury) 100) _asc_cooking_newbury)
        (`AudioComponent.Play` (`self.PreparingPlate1_Cue`) 0.0)))
    (:`then_1`
      (bind _asc_cooking_reginald (cast `/Game/Characters/C_CookingReginald` OtherActor))
      (if (`/Game/Characters/C_CookingReginald.Cut Chicken` _asc_cooking_reginald)
        (set `/Game/Characters/C_CookingReginald.Cut Chicken` false _asc_cooking_reginald)
        (set `/Game/Characters/C_CookingReginald.Empty` true _asc_cooking_reginald)
        (set `/Game/Characters/C_CookingReginald.points` (+ (`/Game/Characters/C_CookingReginald.points` _asc_cooking_reginald) 100) _asc_cooking_reginald)
        (`AudioComponent.Play` (`self.PreparingPlate1_Cue`) 0.0)))
    (:`then_2`
      (bind _asc_cooking_yvonne (cast `/Game/Characters/C_CookingYvonne` OtherActor))
      (if (`/Game/Characters/C_CookingYvonne.SpoonedCaviar` _asc_cooking_yvonne)
        (set `/Game/Characters/C_CookingYvonne.SpoonedCaviar` false _asc_cooking_yvonne)
        (set `/Game/Characters/C_CookingYvonne.Empty` true _asc_cooking_yvonne)
        (set `/Game/Characters/C_CookingYvonne.points` (+ (`/Game/Characters/C_CookingYvonne.points` _asc_cooking_yvonne) 100) _asc_cooking_yvonne)
        (`AudioComponent.Play` (`self.PreparingPlate1_Cue`) 0.0)))
    (:`then_3`
      (bind _asc_cooking_chad (cast `/Game/Characters/C_CookingChad` OtherActor))
      (if (`/Game/Characters/C_CookingChad.ButteredLobster` _asc_cooking_chad)
        (set `/Game/Characters/C_CookingChad.ButteredLobster` false _asc_cooking_chad)
        (set `/Game/Characters/C_CookingChad.Empty` true _asc_cooking_chad)
        (set `/Game/Characters/C_CookingChad.points` (+ (`/Game/Characters/C_CookingChad.points` _asc_cooking_chad) 100) _asc_cooking_chad)
        (`AudioComponent.Play` (`self.PreparingPlate1_Cue`) 0.0)))
    (:`then_4`
      (bind _asc_cooking_jeremia (cast `/Game/Characters/C_CookingJeremia` OtherActor))
      (if (`/Game/Characters/C_CookingJeremia.Cut Cheese` _asc_cooking_jeremia)
        (set `/Game/Characters/C_CookingJeremia.Cut Cheese` false _asc_cooking_jeremia)
        (set `/Game/Characters/C_CookingJeremia.Empty` true _asc_cooking_jeremia)
        (set `/Game/Characters/C_CookingJeremia.points` (+ (`/Game/Characters/C_CookingJeremia.points` _asc_cooking_jeremia) 100) _asc_cooking_jeremia)
        (`AudioComponent.Play` (`self.PreparingPlate1_Cue`) 0.0)))
    (:`then_5`
      (bind _asc_cooking_diana (cast `/Game/Characters/C_CookingDiana` OtherActor))
      (if (`/Game/Characters/C_CookingDiana.Scraped Snails` _asc_cooking_diana)
        (set `/Game/Characters/C_CookingDiana.Scraped Snails` false _asc_cooking_diana)
        (set `/Game/Characters/C_CookingDiana.Empty` true _asc_cooking_diana)
        (set `/Game/Characters/C_CookingDiana.points` (+ (`/Game/Characters/C_CookingDiana.points` _asc_cooking_diana) 100) _asc_cooking_diana)
        (`AudioComponent.Play` (`self.PreparingPlate1_Cue`) 0.0)))))

(fn `UserConstructionScript`)