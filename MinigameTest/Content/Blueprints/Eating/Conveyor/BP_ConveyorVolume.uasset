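; Conveyor belt volume that carries food items (caviar, escargot, pheasant, cheese wheel, lobster, eels) along the actor's forward direction.
; Every tick it queries the Box for overlapping actors of each food class separately and offsets them by Speed scaled by delta time, without sweeping.
; The construction script counter-scales the Arrow so it keeps a constant size when the volume is resized.
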(event `self.ReceiveTick`
  (params (DeltaSeconds :type "Float (single-precision)"))
  (`|ExecutionSequence`
    (:`then_0`
      (for _array_element (`PrimitiveComponent.GetOverlappingActors` (`self.Box`) "/Game/Blueprints/Eating/BP_Caviar.BP_Caviar_C")
        (`self.K2_AddActorWorldOffset` _array_element (* (`KismetMathLibrary.GetForwardVector` (`self.K2_GetActorRotation`)) (* DeltaSeconds (`self.Speed`))) false false)))
    (:`then_1`
      (for _array_element_2 (`PrimitiveComponent.GetOverlappingActors` (`self.Box`) "/Game/Blueprints/Eating/BP_Escargot.BP_Escargot_C")
        (`self.K2_AddActorWorldOffset` _array_element_2 (* (`KismetMathLibrary.GetForwardVector` (`self.K2_GetActorRotation`)) (* DeltaSeconds (`self.Speed`))) false false)))
    (:`then_2`
      (for _array_element_3 (`PrimitiveComponent.GetOverlappingActors` (`self.Box`) "/Game/Blueprints/Eating/BP_Pheasant.BP_Pheasant_C")
        (`self.K2_AddActorWorldOffset` _array_element_3 (* (`KismetMathLibrary.GetForwardVector` (`self.K2_GetActorRotation`)) (* DeltaSeconds (`self.Speed`))) false false)))
    (:`then_3`
      (for _array_element_4 (`PrimitiveComponent.GetOverlappingActors` (`self.Box`) "/Game/Blueprints/Eating/BP_CheeseWheel.BP_CheeseWheel_C")
        (`self.K2_AddActorWorldOffset` _array_element_4 (* (`KismetMathLibrary.GetForwardVector` (`self.K2_GetActorRotation`)) (* DeltaSeconds (`self.Speed`))) false false)))
    (:`then_4`
      (for _array_element_5 (`PrimitiveComponent.GetOverlappingActors` (`self.Box`) "/Game/Blueprints/Eating/BP_Lobster.BP_Lobster_C")
        (`self.K2_AddActorWorldOffset` _array_element_5 (* (`KismetMathLibrary.GetForwardVector` (`self.K2_GetActorRotation`)) (* DeltaSeconds (`self.Speed`))) false false)))
    (:`then_5`
      (for _array_element_6 (`PrimitiveComponent.GetOverlappingActors` (`self.Box`) "/Game/Blueprints/Eating/BP_Eels.BP_Eels_C")
        (`self.K2_AddActorWorldOffset` _array_element_6 (* (`KismetMathLibrary.GetForwardVector` (`self.K2_GetActorRotation`)) (* DeltaSeconds (`self.Speed`))) false false)))))

(fn `UserConstructionScript`
  (`SceneComponent.SetRelativeScale3D` (`self.Arrow`) (/ (1.0 1.0 1.0) (`self.GetActorScale3D`))))