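; Food spawner for the eating conveyor that drops a random dish into the world at its own location.
; BeginPlay starts a looping one-second timer that calls Spawn.
; Spawn rolls a random integer and switches to one of six food actor classes, such as lobster, caviar or escargot, spawning it at reduced scale.
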(event `self.ReceiveBeginPlay`
  (`KismetSystemLibrary.K2_SetTimer` null "Spawn" 1.0 true))

(event `Spawn`
  (switch `int` (`KismetMathLibrary.RandomInteger` 6)
    (:`0`
      (`|SpawnActorFromClass` "/Game/Blueprints/Eating/BP_Lobster.BP_Lobster_C" (`KismetMathLibrary.MakeTransform` (`self.K2_GetActorLocation`) (struct) (`self.Half`)) "Undefined" "OverrideRootScale"))
    (:`1`
      (`|SpawnActorFromClass` "/Game/Blueprints/Eating/BP_CheeseWheel.BP_CheeseWheel_C" (`KismetMathLibrary.MakeTransform` (`self.K2_GetActorLocation`) (struct) (`self.Half`)) "Undefined" "OverrideRootScale"))
    (:`2`
      (`|SpawnActorFromClass` "/Game/Blueprints/Eating/BP_Eels.BP_Eels_C" (`KismetMathLibrary.MakeTransform` (`self.K2_GetActorLocation`) (struct) (`self.Half`)) "Undefined" "OverrideRootScale"))
    (:`3`
      (`|SpawnActorFromClass` "/Game/Blueprints/Eating/BP_Caviar.BP_Caviar_C" (`KismetMathLibrary.MakeTransform` (`self.K2_GetActorLocation`) (struct) (`self.Half`)) "Undefined" "OverrideRootScale"))
    (:`4`
      (`|SpawnActorFromClass` "/Game/Blueprints/Eating/BP_Pheasant.BP_Pheasant_C" (`KismetMathLibrary.MakeTransform` (`self.K2_GetActorLocation`) (struct) (`self.Half`)) "Undefined" "OverrideRootScale"))
    (:`5`
      (`|SpawnActorFromClass` "/Game/Blueprints/Eating/BP_Escargot.BP_Escargot_C" (`KismetMathLibrary.MakeTransform` (`self.K2_GetActorLocation`) (struct) (`self.Half`)) "Undefined" "OverrideRootScale"))))

(fn `UserConstructionScript`)