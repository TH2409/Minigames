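; BP_EatingChad is an eater in an eating game that C_Eating characters feed by bringing carried items into its Box trigger.
; A lobster adds points and plays an eating sound, while any other item deducts a larger amount and plays a disgust sound.
; Each outcome rotates StaticMesh1 through its own timeline, then shares logic that destroys the character's first attached actor and clears its carry flags.
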(event `self.Box.OnComponentBeginOverlap`
  (params (OverlappedComponent :type "PrimitiveComponent Object Reference") (OtherActor :type "Actor Object Reference") (OtherComp :type "PrimitiveComponent Object Reference") (OtherBodyIndex :type Integer) (bFromSweep :type Boolean) (SweepResult :type "HitResult Structure (by ref)"))
  (bind _asc_eating (cast `/Game/Characters/C_Eating` OtherActor :!pure true))
  (if (== (`/Game/Characters/C_Eating.Box` _asc_eating) OtherComp)
    (if (`/Game/Characters/C_Eating.picked up` _asc_eating)
      (if (`/Game/Characters/C_Eating.Lobster` _asc_eating)
        (`|ExecutionSequence`
          (:`then_0`
            (bind (_direction _newtrack_0) (`Timeline|Timeline_0` :!via `PlayFromStart`)
              (:`Update`
                (`SceneComponent.K2_SetRelativeRotation` (`self.StaticMesh1`) (`KismetMathLibrary.MakeRotator` _newtrack_0) false false))))
          (:`then_1`
            (set `self.points` (+ (`self.points`) 100))
            (`self.K2_DestroyActor` (`|GetArrayItem` (`self.GetAttachedActors` _asc_eating)) :!label _label)
            (set `/Game/Characters/C_Eating.picked up` false _asc_eating)
            (set `/Game/Characters/C_Eating.Lobster` false _asc_eating))
          (:`then_2`
            (`AudioComponent.Play` (`self.Char1MEat_Cue`) 0.0)))
        (else
          (`|ExecutionSequence`
            (:`then_0`
              (bind (_direction_2 _newtrack_0_2) (`Timeline|Timeline_1` :!via `PlayFromStart`)
                (:`Update`
                  (`SceneComponent.K2_SetRelativeRotation` (`self.StaticMesh1`) (`KismetMathLibrary.MakeRotator` _newtrack_0_2) false false))))
            (:`then_1`
              (set `self.points` (- (`self.points`) 300))
              (goto _label))
            (:`then_2`
              (`AudioComponent.Play` (`self.Char1MEatDisgust_Cue`) 0.0))))))))

(fn `UserConstructionScript`)