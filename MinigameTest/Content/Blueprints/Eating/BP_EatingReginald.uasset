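; BP_EatingReginald is Reginald, a feeding target in the Eating game that scores items brought by C_Eating.
; When that actor's Box overlaps his Box while it holds an item, its Pheasant flag decides between gaining and losing Points.
; Each outcome plays its own timeline rolling StaticMesh1, prints the score, then destroys the first attached actor and clears PickedUp.
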(event `self.Box.OnComponentBeginOverlap`
  (params (OverlappedComponent :type "PrimitiveComponent Object Reference") (OtherActor :type "Actor Object Reference") (OtherComp :type "PrimitiveComponent Object Reference") (OtherBodyIndex :type Integer) (bFromSweep :type Boolean) (SweepResult :type "HitResult Structure (by ref)"))
  (bind _asc_eating (cast `/Game/Characters/C_Eating` OtherActor :!pure true))
  (if (== (`/Game/Characters/C_Eating.Box` _asc_eating) OtherComp)
    (if (`/Game/Characters/C_Eating.picked up` _asc_eating)
      (if (`/Game/Characters/C_Eating.Pheasant` _asc_eating)
        (`|ExecutionSequence`
          (:`then_0`
            (bind (_direction _newtrack_0) (`Timeline|Timeline_0` :!via `PlayFromStart`)
              (:`Update`
                (`SceneComponent.K2_SetRelativeRotation` (`self.StaticMesh1`) (`KismetMathLibrary.MakeRotator` _newtrack_0) false false))))
          (:`then_1`
            (bind _output_get (set `self.points` (+ (`self.points`) 100)))
            (`KismetSystemLibrary.PrintString` (`KismetStringLibrary.Conv_IntToString` _output_get))
            (`self.K2_DestroyActor` (`|GetArrayItem` (`self.GetAttachedActors` _asc_eating)) :!label _label)
            (set `/Game/Characters/C_Eating.picked up` false _asc_eating)))
        (else
          (`|ExecutionSequence`
            (:`then_0`
              (bind (_direction_2 _newtrack_0_2) (`Timeline|Timeline_1` :!via `PlayFromStart`)
                (:`Update`
                  (`SceneComponent.K2_SetRelativeRotation` (`self.StaticMesh1`) (`KismetMathLibrary.MakeRotator` _newtrack_0_2) false false))))
            (:`then_1`
              (bind _output_get_2 (set `self.points` (- (`self.points`) 300)))
              (`KismetSystemLibrary.PrintString` (`KismetStringLibrary.Conv_IntToString` _output_get_2))
              (goto _label))))))))

(fn `UserConstructionScript`)