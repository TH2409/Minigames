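; Dance pad actor that flashes its emissive lights and changes material colour during play.
; A timeline that replays on finish drives the opacity, cross and plus scalar parameters on the current dynamic material.
; The construction script builds four colour instances and applies a blue monochrome default.
; On BeginPlay, the pad steps once through the four colours at five-second intervals, creating a new dynamic instance each time.
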(event `self.ReceiveBeginPlay`
  (bind _padmaterial (`self.PadMaterial`))
  (`|ExecutionSequence`
    (:`then_0`
      (bind (_direction _lightopacity _lights1 _lights2 _lights3) (`Timeline|Timeline_0` :!label _label)
        (:`Update`
          (`|ExecutionSequence`
            (:`then_0`
              (`MaterialInstanceDynamic.SetScalarParameterValue` _padmaterial "EmissOpacity" _lightopacity))
            (:`then_2`
              (`MaterialInstanceDynamic.SetScalarParameterValue` _padmaterial "Cross" _lights2))
            (:`then_3`
              (`MaterialInstanceDynamic.SetScalarParameterValue` _padmaterial "Plus" _lights3))))
        (:`Finished`
          (`self.Repeat`
            (:`Out`
              (goto _label :!via `PlayFromStart`))))))
    (:`then_1`
      (bind _returnvalue (`PrimitiveComponent.CreateDynamicMaterialInstance` (`self.SM_DancePad`) 0 (`|GetArrayItem` (`self.MaterialColours`))))
      (set `self.PadMaterial` _returnvalue)
      (`KismetSystemLibrary.Delay` 5.0)
      (bind _returnvalue_2 (`PrimitiveComponent.CreateDynamicMaterialInstance` (`self.SM_DancePad`) 0 (`|GetArrayItem` (`self.MaterialColours`) 1)))
      (set `self.PadMaterial` _returnvalue_2)
      (`KismetSystemLibrary.Delay` 5.0)
      (bind _returnvalue_3 (`PrimitiveComponent.CreateDynamicMaterialInstance` (`self.SM_DancePad`) 0 (`|GetArrayItem` (`self.MaterialColours`) 2)))
      (set `self.PadMaterial` _returnvalue_3)
      (`KismetSystemLibrary.Delay` 5.0)
      (bind _returnvalue_4 (`PrimitiveComponent.CreateDynamicMaterialInstance` (`self.SM_DancePad`) 0 (`|GetArrayItem` (`self.MaterialColours`) 3)))
      (set `self.PadMaterial` _returnvalue_4)
      (`KismetSystemLibrary.Delay` 5.0))))

(event `self.ReceiveTick`
  (params (DeltaSeconds :type "Float (single-precision)")))

(fn `UserConstructionScript`
  (bind _sm_dancepad (`self.SM_DancePad`))
  (bind _materialcolours (`self.MaterialColours`))
  (`|ExecutionSequence`
    (:`then_0`
      (bind _returnvalue (`PrimitiveComponent.CreateDynamicMaterialInstance` _sm_dancepad 0 (`|GetArrayItem` _materialcolours)))
      (bind _returnvalue_2 (`PrimitiveComponent.CreateDynamicMaterialInstance` _sm_dancepad 0 (`|GetArrayItem` _materialcolours 1)))
      (bind _returnvalue_3 (`PrimitiveComponent.CreateDynamicMaterialInstance` _sm_dancepad 0 (`|GetArrayItem` _materialcolours 2)))
      (bind _returnvalue_4 (`PrimitiveComponent.CreateDynamicMaterialInstance` _sm_dancepad 0 (`|GetArrayItem` _materialcolours 3)))
      (set `self.MaterialColours` (`|MakeArray` _returnvalue _returnvalue_2 _returnvalue_3 _returnvalue_4)))
    (:`then_1`
      (bind _returnvalue_5 (`PrimitiveComponent.CreateDynamicMaterialInstance` (`self.SM_DancePad`) 0 "/Game/Materials/M_DancePadMonochrome_Blue.M_DancePadMonochrome_Blue"))
      (set `self.PadMaterial` _returnvalue_5)
      (`PrimitiveComponent.SetMaterial` (`self.SM_DancePad`) 0 (`self.PadMaterial`)))))